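; Runner character Blueprint that handles lane switching, game pausing and level UI in a networked game.
; A timeline feeds lane-change update and finish calls whose logic lives outside this graph.
; On pausable levels the authority triggers creation of the HUD and pause menu, which M opens.
; Server-to-multicast events replicate pause state and widget creation, including a named finish screen that pauses the game and disables input.
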(event Custom|MLT_CreatePauseWidget
  (Variables|/Script/Engine.PlayerController|SetbShowMouseCursor (Game|GetPlayerController 0) true)
  (bind _asbp_run_hud (Utilities|Casting|CastToBP_RunHUD (HUD|GetHUD (Game|GetPlayerController 0))))
  (Utilities|IsValid (Variables|/Game/_Game/Blueprints/Widgets/BP_RunHUD.BP_RunHUD_C|GetHUD _asbp_run_hud)
    (:Is%20Valid
      (Widget|SetVisibility (Variables|/Game/_Game/Blueprints/Widgets/BP_RunHUD.BP_RunHUD_C|GetHUD _asbp_run_hud) "Visible"))
    (:Is%20Not%20Valid
      (bind _returnvalue (UserInterface|CreateWidget "/Game/_Game/Blueprints/Widgets/WBP_HUD.WBP_HUD_C"))
      (bind _output_get (Variables|/Game/_Game/Blueprints/Widgets/BP_RunHUD.BP_RunHUD_C|SetHUD _asbp_run_hud _returnvalue))
      (UserInterface|Viewport|AddtoViewport _output_get 0)))
  (if (not (Utilities|IsValid (Variables|Default|GetPauseMenuRef)))
    (bind _returnvalue_2 (UserInterface|CreateWidget "/Game/_Game/Blueprints/Widgets/WBP_PauseMenu.WBP_PauseMenu_C"))
    (bind _output_get_2 (Variables|Default|SetPauseMenuRef _returnvalue_2))
    (UserInterface|Viewport|AddtoViewport _output_get_2 0)))

(event Custom|SVR_CreatePauseWidget
  (CallFunction|MLTCreatePauseWidget))

(event Custom|MLT_SetGamePaused
  (params (IsPaused :type Boolean))
  (Game|SetGamePaused IsPaused))

(event Custom|SVR_SetGamePaused
  (params (IsPaused :type Boolean))
  (CallFunction|MLTSetGamePaused IsPaused))

(event Custom|MLT_Create%20Finish%20Widget
  (params (Name :type String))
  (bind _returnvalue (Game|GetPlayerController 0))
  (bind _returnvalue_2 (UserInterface|CreateWidget "/Game/_Game/Blueprints/Widgets/WBP_FinishWidget_.WBP_FinishWidget__C" (Game|GetPlayerController 0) Name))
  (UserInterface|Viewport|AddtoViewport _returnvalue_2 0)
  (Input|DisableInput _returnvalue)
  (Input|SetInputModeUIOnly _returnvalue _returnvalue_2 "DoNotLock"))

(event EventBeginPlay
  (Utilities|FlowControl|Delay 0.2)
  (Collision|SetCollisionResponsetoChannel (Variables|Character|GetMesh) "ECC_Camera" "ECR_Ignore")
  (Networking|SwitchHasAuthority
    (:Authority
      (bind _asbp_main_level_gm (Utilities|Casting|CastToBP_MainLevel_GM (Game|GetGameMode)))
      (bind _ispausablelevel (Default|IsCurrentLevelPausableLevel _asbp_main_level_gm))
      (if _ispausablelevel
        (CallFunction|SVRCreatePauseWidget)))))

(event EventCreateFinishWidget
  (params (Name :type String))
  (CallFunction|MLTCreateFinishWidget Name)
  (CallFunction|SVRSetGamePaused true))

(event EventChangeLane
  (bind _laneval (Timeline|SwitchLaneTimeline PlayFromStart)
    (:Update
      (Class|RunCharacter|ChangeLaneUpdate _laneval))
    (:Finished
      (Class|RunCharacter|ChangeLaneFinished))))

(event Input|KeyboardEvents|M
  (params (Key :type Key%20Structure :default "None"))
  (:Released
    (CallFunction|ShowPauseMenu)))

(fn ConstructionScript)

(fn ShowPauseMenu
  (bind _returnvalue (Game|GetPlayerController 0))
  (if (Utilities|IsValid (Variables|Default|GetPauseMenuRef))
    (Widget|SetVisibility (Variables|Default|GetPauseMenuRef) "Visible")
    (bind _asbp_run_hud (Utilities|Casting|CastToBP_RunHUD (HUD|GetHUD (Game|GetPlayerController 0))))
    (Widget|SetVisibility (Variables|/Game/_Game/Blueprints/Widgets/BP_RunHUD.BP_RunHUD_C|GetHUD _asbp_run_hud) "Hidden")
    (CallFunction|SVRSetGamePaused true)
    (Variables|/Script/Engine.PlayerController|SetbShowMouseCursor _returnvalue true)
    (Input|SetInputModeUIOnly _returnvalue (Variables|Default|GetPauseMenuRef) "DoNotLock")))